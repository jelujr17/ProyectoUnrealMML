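; BP_Furniture_Antorchas is a placeable torch furniture piece that the player can switch on and off.
; Interact toggles four particle systems together, tracking their state in the OnOff flag, and always returns true.
; EnableInteraction shows or hides the InteractText prompt, and the construction script only calls its parent.
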(event EventEnableInteraction
  (params (enable :type Boolean))
  (Rendering|SetVisibility (Variables|Default|GetInteractText) enable false))

(fn ConstructionScript
  (|CallParentFunction))

(fn Interact
  (if (Variables|Default|GetbOnOff)
    (Components|Activation|Deactivate (Variables|Default|GetParticleSystem1))
    (Variables|Default|SetbOnOff false)
    (else
      (Components|Activation|Activate (Variables|Default|GetParticleSystem) true)
      (Variables|Default|SetbOnOff true)))
  (return true))